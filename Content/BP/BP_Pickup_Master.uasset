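; BP_Pickup_Master is a base pickup actor, collected through an Interract event when the third-person character is in range.
; Sphere overlaps with that character toggle CanIteract, and the end overlap, not the begin, sets the character's LastInteractObj to this pickup.
; When allowed, Interract calls the empty Body event, apparently a hook for child pickups, then destroys the actor and prints a collection message.
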(event OnComponentEndOverlap(Sphere)
  (params (OverlappedComponent :type Primitive%20Component%20Object%20Reference) (OtherActor :type Actor%20Object%20Reference) (OtherComp :type Primitive%20Component%20Object%20Reference) (OtherBodyIndex :type Integer))
  (bind _asbp_third_person_character (Utilities|Casting|CastToBP_ThirdPersonCharacter OtherActor))
  (Variables|/Game/ThirdPerson/Blueprints/BP_ThirdPersonCharacter.BP_ThirdPersonCharacter_C|SetLastInteractObj _asbp_third_person_character self)
  (Variables|Default|SetCan%20Iteract? false))

(event OnComponentBeginOverlap(Sphere)
  (params (OverlappedComponent :type Primitive%20Component%20Object%20Reference) (OtherActor :type Actor%20Object%20Reference) (OtherComp :type Primitive%20Component%20Object%20Reference) (OtherBodyIndex :type Integer) (bFromSweep :type Boolean) (SweepResult :type Hit%20Result%20Structure%20%28by%20ref%29))
  (Utilities|Casting|CastToBP_ThirdPersonCharacter OtherActor)
  (Variables|Default|SetCan%20Iteract? true))

(event Custom|Body)

(event EventInterract
  (if (Variables|Default|GetCan%20Iteract?)
    (CallFunction|Body)
    (Actor|DestroyActor)
    (Development|PrintString "ITEN COLETADO")))

(fn ConstructionScript)