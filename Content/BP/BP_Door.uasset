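; BP_Door is a key-locked door that swings open when something overlaps its Box trigger while HasKey is true.
; A Timeline curve drives the StaticMesh's relative yaw, and its Finished pin sets DoorOpen from the final curve value.
; End overlap reverses the Timeline only if DoorOpen is set, so leaving mid-swing does not close it.
; The Interract event is empty, and a leftover collapsed debug graph never runs.
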(event OnComponentBeginOverlap(Box)
  (params (OverlappedComponent :type Primitive%20Component%20Object%20Reference) (OtherActor :type Actor%20Object%20Reference) (OtherComp :type Primitive%20Component%20Object%20Reference) (OtherBodyIndex :type Integer) (bFromSweep :type Boolean) (SweepResult :type Hit%20Result%20Structure%20%28by%20ref%29))
  (if (Variables|Gameplay|GetHasKey?)
    (if (not (Variables|Gameplay|GetDoorOpen?))
      (bind _moviment_door (Timeline|Timeline PlayFromStart)
        (:Update
          (Transformation|SetRelativeRotation (Variables|Default|GetStaticMesh) (Math|Rotator|MakeRotator 0.0 0.0 _moviment_door) false false))
        (:Finished
          (Variables|Gameplay|SetDoorOpen? (> _moviment_door 0.0)))))))

(event OnComponentEndOverlap(Box)
  (params (OverlappedComponent :type Primitive%20Component%20Object%20Reference) (OtherActor :type Actor%20Object%20Reference) (OtherComp :type Primitive%20Component%20Object%20Reference) (OtherBodyIndex :type Integer))
  (if (Variables|Gameplay|GetDoorOpen?)
    (bind _moviment_door (Timeline|Timeline ReverseFromEnd)
      (:Update
        (Transformation|SetRelativeRotation (Variables|Default|GetStaticMesh) (Math|Rotator|MakeRotator 0.0 0.0 _moviment_door) false false))
      (:Finished
        (Variables|Gameplay|SetDoorOpen? (> _moviment_door 0.0))))))

(event EventInterract)

(fn ConstructionScript)